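; BP_OceanFloater is an actor meant to float on ocean waves, but its height update is unfinished.
; Each tick it draws the ocean material to a render target, then samples that target at its XY position.
; The SetActorLocation that would turn the blue channel and WaveHeight into Z is disconnected, so the actor never moves.
; WorldToOceanScale's modulo-based tiling math is also unconnected to any output.
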(event `self.ReceiveTick`
  (params (DeltaSeconds :type "Float (single-precision)"))
  (`KismetRenderingLibrary.DrawMaterialToRenderTarget` (`self.RenderTarget`) (`self.OceanMat`))
  (`self.FloatToHeight`))

(fn `FloatToHeight`
  (bind _returnvalue (`KismetRenderingLibrary.ReadRenderTargetUV` (`self.RenderTarget`) (`self.WorldToOceanScale` (.x (`self.K2_GetActorLocation`))) (`self.WorldToOceanScale` (.y (`self.K2_GetActorLocation`))))))

(fn `TrueModulo`
  (params (Dividend :type Integer) (Divisor :type Integer))
  (returns (Result :type Integer))
  (if (>= Dividend 0)
    (return (mod Dividend Divisor))
    (else
      (return (mod (+ Dividend 10000000) Divisor)))))

(fn `UserConstructionScript`)