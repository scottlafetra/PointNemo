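; BP_OceanTiler keeps a square grid of BP_Ocean tiles centred on its own position, so the ocean follows it as it moves.
; On BeginPlay it spawns TilesDiameter squared tiles into an array.
; Every Tick it repositions them around its X/Y location, truncated to multiples of UnitDistance, so tiles jump in whole-tile steps at Z zero.
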(event `self.ReceiveBeginPlay`
  (if (not (`self.TilesCreated`))
    (`self.CreateTiles`)))

(event `self.ReceiveTick`
  (params (DeltaSeconds :type "Float (single-precision)"))
  (`self.UpdateTiles`))

(fn `CreateTiles`
  (bind _tilesdiameter (`self.TilesDiameter`))
  (for _index (range (* _tilesdiameter _tilesdiameter))
    (bind _returnvalue (`|SpawnActorFromClass` "/Game/Blueprints/BP_Ocean.BP_Ocean_C" (`self.GetTransform`) "Undefined" "OverrideRootScale" null null))
    (`KismetArrayLibrary.Array_Add` (`self.Tiles`) _returnvalue))
  (set `self.TilesCreated` true)
  (`self.UpdateTiles`))

(fn `UpdateTiles`
  (locals (TileRadius :type Integer :default 0))
  (bind _unitdistance (`self.UnitDistance`))
  (bind _unitdistance_2 (`self.UnitDistance`))
  (set `local.TileRadius` (/ (`self.TilesDiameter`) 2))
  (for _index (range (`self.TilesDiameter`))
    (for _index_2 (range (`self.TilesDiameter`))
      (`self.K2_SetActorLocation` (`|GetArrayItem` (`self.Tiles`) (+ _index_2 (* _index (`self.TilesDiameter`)))) (`KismetMathLibrary.MakeVector` (+ (* (`KismetMathLibrary.FTrunc` (/ (.x (`self.K2_GetActorLocation`)) _unitdistance_2)) _unitdistance_2) (* (- _index_2 (`local.TileRadius`)) (`self.UnitDistance`))) (+ (* (`KismetMathLibrary.FTrunc` (/ (.y (`self.K2_GetActorLocation`)) _unitdistance)) _unitdistance) (* (- _index (`local.TileRadius`)) (`self.UnitDistance`)))) false false))))

(fn `UserConstructionScript`)