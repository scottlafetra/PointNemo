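; MultiplayerTest is a debug Blueprint for inspecting the players in a multiplayer session.
; On every Tick it loops over the Game State's PlayerArray and prints each player's name, ping and spectator flag with Print String.
; BeginPlay, ActorBeginOverlap and the construction script are empty.
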(event `self.ReceiveTick`
  (params (DeltaSeconds :type "Float (single-precision)"))
  (for _array_element (`GameStateBase.PlayerArray` (`GameplayStatics.GetGameState`))
    (`KismetSystemLibrary.PrintString` (`KismetTextLibrary.Conv_TextToString` (`|FormatText` "{Name} | {Ping} | Spectator: {Spec}" (`KismetTextLibrary.Conv_StringToText` (`PlayerState.GetPlayerName` _array_element)) (`PlayerState.Ping` _array_element) (`KismetTextLibrary.Conv_BoolToText` (`PlayerState.bIsSpectator` _array_element)))) true true (struct :`G` 0.66 :`B` 1.0 :`A` 1.0) 0.0)))

(fn `UserConstructionScript`)