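; TestFloatBox is a test actor that keeps itself from sinking below world height zero.
; Each Tick it checks its Z location and, when negative, moves itself back to Z zero without sweeping, preserving X and Y.
; Unreachable ThrustStrength setters and an unused depth-scaled expression remain in the graph but have no effect.
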(event `self.ReceiveTick`
  (params (DeltaSeconds :type "Float (single-precision)"))
  (if (< (.z (`self.K2_GetActorLocation`)) 0.0)
    (`self.K2_SetActorLocation` (`KismetMathLibrary.MakeVector` (.x (`self.K2_GetActorLocation`)) (.y (`self.K2_GetActorLocation`))))))

(fn `UserConstructionScript`)