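; BP_Debris2_7 is a debris variant that extends a parent Blueprint with its own float points.
; On BeginPlay it runs the parent logic, then appends Float2 and Float3 to the FloatPoints array.
; It adds no other logic: Tick and overlap events are disabled stubs, and the construction script only calls the parent.
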(event `self.ReceiveBeginPlay`
  (`parent.ReceiveBeginPlay`)
  (for _array_element (`|MakeArray` (`self.Float 2`) (`self.Float 3`))
    (`KismetArrayLibrary.Array_Add` (`self.FloatPoints`) _array_element)))

(fn `UserConstructionScript`
  (`parent.UserConstructionScript`))