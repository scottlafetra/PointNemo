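; BP_OceanRenderer renders an ocean material to a render target and serves panning wave heights by UV.
; InitHeightMap draws the target once and sizes a flat array as the height cache.
; GetHeightAtUV offsets UVs by time, lazily filling empty (zero) entries from the target's blue channel scaled by WaveHeight.
; BeginPlay pre-samples a small UV grid, using a delayed-loop macro to spread reads across frames.
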(event `self.ReceiveBeginPlay`
  (`self.InitHeightMap`)
  ;[0.9387 0.0382 0.0382] Caches a 100x100 version of the rendertarget asyncronoulsy
  (bind _index (`self.ForLoopDelay` 0 10 :!label _label)
    (:`Body`
      (for _index_2 (range 11)
        (`self.GetHeightAtUV` (/ (`KismetMathLibrary.Conv_IntToDouble` _index_2) 1000.0) (/ (`KismetMathLibrary.Conv_IntToDouble` _index) 1000.0))))
    (:`DelayOut`
      (`KismetSystemLibrary.Delay` 0.0)
      (goto _label :!via `DelayIn`))))

(event `self.ReceiveTick`
  (params (DeltaSeconds :type "Float (single-precision)")))

(fn `GetHeightAtUV`
  (params (U :type "Float (double-precision)") (V :type "Float (double-precision)"))
  (returns (`Wave Height` :type "Float (double-precision)"))
  (bind _oceanwidth (`self.OceanWidth`))
  (bind _returnvalue (* (`self.PanSpeed`) (`GameplayStatics.GetTimeSeconds`)))
  (bind _returnvalue_2 (mod (+ V _returnvalue) 1.0))
  (bind _returnvalue_3 (mod (+ U _returnvalue) 1.0))
  (bind _returnvalue_4 (+ (* (`KismetMathLibrary.FTrunc` (* _oceanwidth _returnvalue_3)) _oceanwidth) (`KismetMathLibrary.FTrunc` (* _oceanwidth _returnvalue_2))))
  (bind _output (`|GetArrayItem` (`self.HeightMap`) _returnvalue_4))
  (if (!= _output 0.0)
    (return _output)
    (else
      (bind _returnvalue_5 (`KismetRenderingLibrary.ReadRenderTargetUV` (`self.OceanRT`) _returnvalue_3 _returnvalue_2))
      (bind _returnvalue_6 (* (/ (`KismetMathLibrary.Conv_ByteToDouble` (`.B` (break `Color` _returnvalue_5))) 256.0) (`self.WaveHeight`)))
      (`KismetArrayLibrary.Array_Set` (`self.HeightMap`) _returnvalue_4 _returnvalue_6)
      (return _returnvalue_6))))

(fn `InitHeightMap`
  (if (not (`self.HeightMapMade`))
    (set `self.HeightMapMade` true)
    (`KismetArrayLibrary.Array_Clear` (`self.HeightMap`))
    (`KismetRenderingLibrary.DrawMaterialToRenderTarget` (`self.OceanRT`) (`self.OceanMat`))
    (`KismetArrayLibrary.Array_Resize` (`self.HeightMap`) (* (`self.OceanWidth`) (`self.OceanWidth`)))))

(fn `UserConstructionScript`)