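; BP_Bag is a bag Blueprint that registers float points for itself, apparently for buoyancy handled outside this graph.
; On BeginPlay it calls the parent, then adds the relative locations of three FloatThing components to the FloatPoints array.
; Overlap and Tick are disabled stubs, and the construction script only calls the parent.
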(event `self.ReceiveBeginPlay`
  (`parent.ReceiveBeginPlay`)
  (for _array_element (`|MakeArray` (`self.Float thing 2`) (`self.Float thing 3`) (`self.Float Thing 4`))
    (`KismetArrayLibrary.Array_Add` (`self.FloatPoints`) (`SceneComponent.RelativeLocation` _array_element))))

(fn `UserConstructionScript`
  (`parent.UserConstructionScript`))